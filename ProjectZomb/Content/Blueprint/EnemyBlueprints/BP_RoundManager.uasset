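; BP_RoundManager runs wave-based enemy rounds and registers itself on BP_GameInstance.
; A delayed, self-calling EnemyCheck triggers random entries in ActiveSpawns while alive and remaining-spawn counts allow, and completes the round when both run out.
; RoundComplete garbage-collects, updates the player's round widget, and sets the next spawn count by round number, switching to a multiplier-based count from round ten.
; Interface events adjust both enemy counters and restart the check.
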(event `self.ReceiveBeginPlay`
  ;[1 1 1] Instance reference initialised
  (bind _asbp_game_instance (cast `/Game/FirstPerson/Blueprints/BP_GameInstance` (`GameplayStatics.GetGameInstance`)))
  (set `/Game/FirstPerson/Blueprints/BP_GameInstance.ref_roundManager` self _asbp_game_instance)
  (`KismetSystemLibrary.Delay` 5.0)
  (`self.Event EnemyCheck`))

(event `Event EnemyCheck`
  ;[1 1 1] If max enemy count not yet reached, enemy spawned at random location
  (`KismetSystemLibrary.Delay` 1.0)
  (if (and (< (`self.aliveEnemies`) (`self.maxEnemies`)) (> (`self.enemiesToSpawn`) 0))
    (bind _values (`BlueprintMapLibrary.Map_Values` (`self.activeSpawns`)))
    (`/Game/Blueprint/EnemyBlueprints/BP_EnemySpawn.Event SpawnEnemy` (`KismetArrayLibrary.Array_Random` _values))
    (`self.Event EnemyCheck`)
    (elif (and (<= (`self.enemiesToSpawn`) 0) (== (`self.aliveEnemies`) 0))
      (`self.Event Round Complete`))))

(event `Event Round Complete`
  (bind _currentround (`self.currentRound`))
  ;[1 1 1] Update round counter
  (`KismetSystemLibrary.CollectGarbage`)
  (`KismetSystemLibrary.Delay` 5.0)
  ;[1 1 1] UI Updated
  (`/Engine/EditorBlueprintResources/StandardMacros.IncrementInt` _currentround
    (:`  `
      (bind _asbp_first_person_character (cast `/Game/FirstPerson/Blueprints/BP_FirstPersonCharacter` (`GameplayStatics.GetPlayerCharacter` 0)))
      (`/Game/Blueprint/Widgets/W_PlayerUI.Event UpdateRound` (`/Game/FirstPerson/Blueprints/BP_FirstPersonCharacter.ref_playerWidget` _asbp_first_person_character) _currentround)
      ;[1 1 1] calc enemies to spawn based on round (below round ten, count increases linearly)
      (if (< _currentround 10)
        (bind _result (`/Engine/EditorBlueprintResources/StandardMacros.DecrementInt` (* (`self.currentRound`) 4))
          (:`  `
            (set `self.enemiesToSpawn` _result)))
        (else
          (set `self.enemiesToSpawn` (`KismetMathLibrary.Round` (* 40.0 (`self.waveMultiplier`))))))
      ;[1 1 1] Begin spawning enemies
      (`self.Event EnemyCheck`))))

(event `/Game/Blueprint/EnemyBlueprints/BPI_RoundManager.updateAliveEnemies`
  (params (Increment :type Boolean))
  (bind _aliveenemies (`self.aliveEnemies`))
  ;[1 1 1] Interface functions
  (if Increment
    (`/Engine/EditorBlueprintResources/StandardMacros.IncrementInt` _aliveenemies)
    (else
      (`/Engine/EditorBlueprintResources/StandardMacros.DecrementInt` _aliveenemies))))

(event `/Game/Blueprint/EnemyBlueprints/BPI_RoundManager.updateEnemsToSpawn`
  (params (increment :type Boolean))
  (bind _enemiestospawn (`self.enemiesToSpawn`))
  ;[1 1 1] Interface functions
  (if increment
    (`/Engine/EditorBlueprintResources/StandardMacros.IncrementInt` _enemiestospawn)
    (else
      (`/Engine/EditorBlueprintResources/StandardMacros.DecrementInt` _enemiestospawn))))

(event `/Game/Blueprint/EnemyBlueprints/BPI_RoundManager.enemyCheck`
  ;[1 1 1] Interface functions
  (`self.Event EnemyCheck`))

(fn `getRound`
  (returns (currRound :type Integer))
  (return (`self.currentRound`)))

(fn `UserConstructionScript`)