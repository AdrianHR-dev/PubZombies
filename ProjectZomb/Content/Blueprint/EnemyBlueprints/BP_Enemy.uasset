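; Round-based enemy that enters the map, chases the player and damages them on contact, with a one-second cooldown.
; Health and walk speed depend on the round read from the actor tagged "rManager".
; Collision zone stays off until it reaches its start location; Tick then reissues AIMoveTo toward the player.
; DamageEnemy awards score for hits and kills, updating the manager's alive count and triggering its enemy check on death.
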(event `self.ReceiveBeginPlay`
  (bind _charactermovement (`self.CharacterMovement`))
  ;[1 1 1] Initialisation of enemy
  (`PrimitiveComponent.SetCollisionEnabled` (`self.EnemyCollisionZone`) "NoCollision")
  (bind _outactors (`GameplayStatics.GetAllActorsWithTag` "rManager"))
  (bind _output (`|GetArrayItem` _outactors))
  (message `/Game/Blueprint/EnemyBlueprints/BPI_RoundManager.updateAliveEnemies` _output true)
  (message `/Game/Blueprint/EnemyBlueprints/BPI_RoundManager.updateEnemsToSpawn` _output false)
  (bind _currround (message `/Game/Blueprint/EnemyBlueprints/BPI_RoundManager.getRound` _output))
  ;[1 1 1] Enemy spanw speed setting
  (set `self.Health` (* (`self.Health`) (* _currround (`self.healthMultiplier`))))
  (if (>= _currround 10)
    (set `CharacterMovementComponent.MaxWalkSpeed` 450.0 _charactermovement)
    (elif (== _currround 1)
      (set `CharacterMovementComponent.MaxWalkSpeed` 60.0 _charactermovement)
      (else
        (set `CharacterMovementComponent.MaxWalkSpeed` (`KismetMathLibrary.Conv_IntToDouble` (+ (* (`KismetMathLibrary.RandomInteger` (- _currround 1)) 50) 50)) _charactermovement))))
  ;[1 1 1] Enemy first moves to required location to spawn before chasing player
  (`|AIMoveTo` self (`self.startLocation`) null 25.0
    (:`OnSuccess`
      (set `self.inMap` true)
      (`PrimitiveComponent.SetCollisionEnabled` (`self.EnemyCollisionZone`) "QueryAndPhysics"))))

(event `self.ReceiveTick`
  (params (DeltaSeconds :type "Float (single-precision)"))
  ;[1 1 1] Move enemy to player
  (if (`self.inMap`)
    (`|AIMoveTo` self (0.0 0.0 0.0) (`GameplayStatics.GetPlayerCharacter` 0) 0.0 true)))

(event `/Game/Blueprint/EnemyBlueprints/BPI_Enemy.DamageEnemy`
  (params (DamageDone :type "Float (double-precision)"))
  (bind _returnvalue (`GameplayStatics.GetPlayerCharacter` 0))
  (bind _returnvalue_2 (`GameplayStatics.GetPlayerCharacter` 0))
  ;[1 1 1] Events to perform when enemy takes damage
  ;[1 1 1] Enemy takes damage
  (bind _output_get (set `self.Health` (- (`self.Health`) DamageDone)))
  ;[1 1 1] If no health left, destroy enemy
  (if (<= _output_get 0.0)
    ;[1 1 1] Enemy alive count decreased; check whether to spawn new one
    (bind _outactors (`GameplayStatics.GetAllActorsWithTag` "rManager"))
    (bind _output (`|GetArrayItem` _outactors))
    (message `/Game/Blueprint/EnemyBlueprints/BPI_RoundManager.updateAliveEnemies` _output false)
    (message `/Game/Blueprint/EnemyBlueprints/BPI_RoundManager.enemyCheck` _output)
    ;[1 1 1] Player score incremented by 50 for a kill
    (bind _currscore (message `/Game/FirstPerson/Blueprints/BPI_PlayerCharacter.getScore` _returnvalue))
    (message `/Game/FirstPerson/Blueprints/BPI_PlayerCharacter.setScore` _returnvalue (+ _currscore 50))
    (`self.K2_DestroyActor`)
    (else
      ;[1 1 1] Player score incremented by 10 for a hit
      (bind _currscore_2 (message `/Game/FirstPerson/Blueprints/BPI_PlayerCharacter.getScore` _returnvalue_2))
      (message `/Game/FirstPerson/Blueprints/BPI_PlayerCharacter.setScore` _returnvalue_2 (+ _currscore_2 10)))))

(event `self.ReceiveHit`
  (params (MyComp :type "PrimitiveComponent Object Reference") (Other :type "Actor Object Reference") (OtherComp :type "PrimitiveComponent Object Reference") (bSelfMoved :type Boolean) (HitLocation :type "Vector Structure") (HitNormal :type "Vector Structure") (NormalImpulse :type "Vector Structure") (Hit :type "HitResult Structure (by ref)"))
  ;[1 1 1] Damage player on collision
  (if (and (== Other (`GameplayStatics.GetPlayerCharacter` 0)) (== (`self.attacking`) false))
    (set `self.attacking` true)
    (message `/Game/FirstPerson/Blueprints/BPI_PlayerCharacter.takeDamage` (`GameplayStatics.GetPlayerCharacter` 0))
    (`KismetSystemLibrary.Delay` 1.0)
    (set `self.attacking` false)))

(fn `UserConstructionScript`)