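; BP_EnemySpawn is a named enemy spawn point that creates BP_Enemy actors.
; On BeginPlay it registers itself in the BP_GameInstance SpawnPoints map under its SpawnName.
; Its SpawnEnemy event spawns an enemy just below the actor, ignoring collision, and passes the EntryPoint component's world location as the enemy's StartLocation.
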(event `self.ReceiveBeginPlay`
  (bind _asbp_game_instance (cast `/Game/FirstPerson/Blueprints/BP_GameInstance` (`GameplayStatics.GetGameInstance`)))
  (bind _output_get (set `self.ref_gameInstance` _asbp_game_instance))
  (`BlueprintMapLibrary.Map_Add` (`/Game/FirstPerson/Blueprints/BP_GameInstance.spawnPoints` _output_get) (`self.SpawnName`) self))

(event `Event SpawnEnemy`
  (bind (_returnvalue_x _returnvalue_y _returnvalue_z) (`KismetMathLibrary.BreakVector` (`self.K2_GetActorLocation`)))
  ;[1 1 1] Spawn enemy just below spawn point
  (`|SpawnActorFromClass` "/Game/Blueprint/EnemyBlueprints/BP_Enemy.BP_Enemy_C" (`KismetMathLibrary.MakeTransform` (`KismetMathLibrary.MakeVector` _returnvalue_x _returnvalue_y (- _returnvalue_z 200.0))) "AlwaysSpawn" "MultiplyWithRoot" null (`SceneComponent.K2_GetComponentLocation` (`self.entryPoint`)) null))

(fn `UserConstructionScript`)